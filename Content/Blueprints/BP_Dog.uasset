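; BP_Dog is a dog Blueprint that prints its state to the screen on key presses.
; E loops over the Items array and prints the display name of each entry.
; P prints the PScore and Health values.
; The event graph only reads these variables, and the construction script is empty.
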(event Input|KeyboardEvents|E
  (params (Key :type Key%20Structure :default "None"))
  (:Pressed
    (for _array_element (Variables|Default|GetItems)
      (Development|PrintString (Utilities|GetDisplayName _array_element) true true "(R=1.000000,G=0.000000,B=0.000000,A=1.000000)" 1e+01))))

(event Input|KeyboardEvents|P
  (params (Key :type Key%20Structure :default "None"))
  (:Pressed
    (Development|PrintString (Utilities|String|ToString(Integer) (Variables|Default|GetPScore)))
    (Development|PrintString (Utilities|String|ToString(Integer) (Variables|Default|GetHealth)))))

(fn ConstructionScript)